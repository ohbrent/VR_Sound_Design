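; BP_ChordObject is an actor that lets the VR player switch chord flow by overlapping trigger boxes.
; Four boxes (CGAMF, DM7, Am7, Free) each write a ChordFlowType to the VR pawn's GameControllerComponent, with the pawn cached at BeginPlay.
; The three chord boxes also reset PlayTime and raise ResetFlag, while Free only changes the type.
; PreviousChordFlowType is overwritten before its check, so that guard always passes.
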(event OnComponentBeginOverlap(boxCGAMF)
  (params (OverlappedComponent :type Primitive%20Component%20Object%20Reference) (OtherActor :type Actor%20Object%20Reference) (OtherComp :type Primitive%20Component%20Object%20Reference) (OtherBodyIndex :type Integer) (bFromSweep :type Boolean) (SweepResult :type Hit%20Result%20Structure%20%28by%20ref%29))
  (bind _as_vrpawn (Variables|Default|GetAs%20VRPawn))
  (bind _gamecontrollercomponent (Variables|/Game/VRTemplate/Blueprints/VRPawn.VRPawn_C|GetGameControllerComponent _as_vrpawn))
  (Variables|/Game/Custom_BP/GameControllerComponent.GameControllerComponent_C|SetChordFlowType _gamecontrollercomponent 0)
  (Variables|Default|SetPreviousChordFlowType 0)
  (if (not (== (Variables|Default|GetPreviousChordFlowType) 3))
    (Variables|/Game/Custom_BP/GameControllerComponent.GameControllerComponent_C|SetPlayTime _gamecontrollercomponent 0.0)
    (Variables|/Game/Custom_BP/GameControllerComponent.GameControllerComponent_C|SetResetFlag _gamecontrollercomponent true)))

(event OnComponentBeginOverlap(boxDM7)
  (params (OverlappedComponent :type Primitive%20Component%20Object%20Reference) (OtherActor :type Actor%20Object%20Reference) (OtherComp :type Primitive%20Component%20Object%20Reference) (OtherBodyIndex :type Integer) (bFromSweep :type Boolean) (SweepResult :type Hit%20Result%20Structure%20%28by%20ref%29))
  (bind _as_vrpawn (Variables|Default|GetAs%20VRPawn))
  (bind _gamecontrollercomponent (Variables|/Game/VRTemplate/Blueprints/VRPawn.VRPawn_C|GetGameControllerComponent _as_vrpawn))
  (Variables|/Game/Custom_BP/GameControllerComponent.GameControllerComponent_C|SetChordFlowType _gamecontrollercomponent 1)
  (Variables|Default|SetPreviousChordFlowType 1)
  (if (not (== (Variables|Default|GetPreviousChordFlowType) 3))
    (Variables|/Game/Custom_BP/GameControllerComponent.GameControllerComponent_C|SetPlayTime _gamecontrollercomponent 0.0)
    (Variables|/Game/Custom_BP/GameControllerComponent.GameControllerComponent_C|SetResetFlag _gamecontrollercomponent true)))

(event OnComponentBeginOverlap(boxAm7)
  (params (OverlappedComponent :type Primitive%20Component%20Object%20Reference) (OtherActor :type Actor%20Object%20Reference) (OtherComp :type Primitive%20Component%20Object%20Reference) (OtherBodyIndex :type Integer) (bFromSweep :type Boolean) (SweepResult :type Hit%20Result%20Structure%20%28by%20ref%29))
  (bind _as_vrpawn (Variables|Default|GetAs%20VRPawn))
  (bind _gamecontrollercomponent (Variables|/Game/VRTemplate/Blueprints/VRPawn.VRPawn_C|GetGameControllerComponent _as_vrpawn))
  (Variables|/Game/Custom_BP/GameControllerComponent.GameControllerComponent_C|SetChordFlowType _gamecontrollercomponent 2)
  (Variables|Default|SetPreviousChordFlowType 2)
  (if (not (== (Variables|Default|GetPreviousChordFlowType) 3))
    (Variables|/Game/Custom_BP/GameControllerComponent.GameControllerComponent_C|SetPlayTime _gamecontrollercomponent 0.0)
    (Variables|/Game/Custom_BP/GameControllerComponent.GameControllerComponent_C|SetResetFlag _gamecontrollercomponent true)))

(event OnComponentBeginOverlap(boxFree)
  (params (OverlappedComponent :type Primitive%20Component%20Object%20Reference) (OtherActor :type Actor%20Object%20Reference) (OtherComp :type Primitive%20Component%20Object%20Reference) (OtherBodyIndex :type Integer) (bFromSweep :type Boolean) (SweepResult :type Hit%20Result%20Structure%20%28by%20ref%29))
  (Variables|/Game/Custom_BP/GameControllerComponent.GameControllerComponent_C|SetChordFlowType (Variables|/Game/VRTemplate/Blueprints/VRPawn.VRPawn_C|GetGameControllerComponent (Variables|Default|GetAs%20VRPawn)) 3)
  (Variables|Default|SetPreviousChordFlowType 3))

(event EventBeginPlay
  (bind _asvrpawn (Utilities|Casting|CastToVRPawn (Game|Player|GetPlayerPawn 0)))
  (Variables|Default|SetAs%20VRPawn _asvrpawn))

(fn ConstructionScript)