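; BP_ReplayEffact is a short-lived visual effect actor with a Sphere component and a tintable Niagara effect.
; Each Tick applies a constant upward force to the Sphere and adds delta time to a Timer, destroying the actor once it reaches two seconds.
; SetEffectColor builds a color from R, G and B values and passes it to the Niagara component's Color variable.
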(event EventBeginPlay)

(event Collision|EventActorBeginOverlap
  (params (OtherActor :type Actor%20Object%20Reference)))

(event EventTick
  (params (DeltaSeconds :type Float%20%28single-precision%29))
  (Physics|AddForce (Variables|Default|GetSphere) "0.000000,0.000000,70.000000" "None" false)
  (Variables|Default|SetTimer (+ (Variables|Default|GetTimer) DeltaSeconds))
  (if (>= (Variables|Default|GetTimer) 2.0)
    (Actor|DestroyActor)))

(fn ConstructionScript)

(fn SetEffectColor
  (params (R :type Float%20%28double-precision%29) (G :type Float%20%28double-precision%29) (B :type Float%20%28double-precision%29))
  (Niagara|SetNiagaraVariable(LinearColor) (Variables|Default|GetNiagara) "Color" (Math|Color|MakeColor R G B)))