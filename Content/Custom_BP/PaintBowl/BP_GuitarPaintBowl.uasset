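; Guitar paint bowl for the VR painting feature that switches the player's brush sound to guitar.
; Caches the VRPawn on BeginPlay, then reacts when a component named "Bodypart2" overlaps its box collision.
; The overlap sets the brush sound type on the pawn's GameControllerComponent, plays a guitar note and spawns a yellow-tinted Niagara effect at the bowl.
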(event OnComponentBeginOverlap(BoxCollision)
  (params (OverlappedComponent :type Primitive%20Component%20Object%20Reference) (OtherActor :type Actor%20Object%20Reference) (OtherComp :type Primitive%20Component%20Object%20Reference) (OtherBodyIndex :type Integer) (bFromSweep :type Boolean) (SweepResult :type Hit%20Result%20Structure%20%28by%20ref%29))
  (bind _bowl_root_ (Variables|Default|GetBowl%28Root%29))
  (bind _returnvalue (Transformation|GetWorldLocation _bowl_root_))
  (if (Utilities|Enum|Equal(Enum) (Utilities|GetObjectName OtherComp) "Bodypart2")
    (Variables|/Game/Custom_BP/GameControllerComponent.GameControllerComponent_C|SetBrushSoundType (Variables|/Game/VRTemplate/Blueprints/VRPawn.VRPawn_C|GetGameControllerComponent (Variables|Default|GetAs%20VRPawn)) 2)
    (Audio|PlaySoundatLocation "/Game/Imported/Guitar/Guitar_C3.Guitar_C3" _returnvalue "0, 0, 0" 1.0 1.0 0.0 0 0 0 0)
    (bind _returnvalue_2 (Niagara|SpawnSystematLocation "/Game/NiaigaraEffect/NS_PaintBowl.NS_PaintBowl" _returnvalue))
    (Niagara|SetNiagaraVariable(LinearColor) _returnvalue_2 "Color" (Math|Color|MakeColor 1.0 1.0 0.0))))

(event EventBeginPlay
  (bind _asvrpawn (Utilities|Casting|CastToVRPawn (Game|Player|GetPlayerPawn 0)))
  (Variables|Default|SetAs%20VRPawn _asvrpawn))

(event EventTick
  (params (DeltaSeconds :type Float%20%28single-precision%29)))

(fn ConstructionScript)