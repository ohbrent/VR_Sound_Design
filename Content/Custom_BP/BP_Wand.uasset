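; VR wand that, while held, scrubs song playback and fires BP_Shootable projectiles.
; Tick line-traces along the wand, placing the NSWandEnd effect at the hit.
; Hitting a component named "Torus" pauses play and converts the hit angle into PlayTime on the pawn's GameControllerComponent; other hit components resume play.
; Left index curl launches projectiles by impulse, while SpawnObject, which creates sound objects by MeshIndex, is unconnected.
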(event Input|EnhancedActionEvents|EnhancedInputActionIA_Hand_IndexCurl_Left
  (params (ActionValue :type Float%20%28double-precision%29) (ElapsedSeconds :type Float%20%28double-precision%29) (TriggeredSeconds :type Float%20%28double-precision%29) (InputAction :type Input%20Action%20Object%20Reference :default "/Game/VRTemplate/Input/Actions/Hands/IA_Hand_IndexCurl_Left.IA_Hand_IndexCurl_Left"))
  (bind _staticmesh_rootcomponent_ (Variables|Default|GetStaticMesh%28RootComponent%29))
  (bind _returnvalue (Transformation|GetWorldLocation _staticmesh_rootcomponent_))
  (bind _returnvalue_2 (Transformation|GetWorldLocation _staticmesh_rootcomponent_))
  (bind _returnvalue_3 (Transformation|GetWorldRotation _staticmesh_rootcomponent_))
  (bind _returnvalue_4 (* _returnvalue_3 -1e+02))
  (bind _returnvalue_5 (+ _returnvalue _returnvalue_4))
  (bind _returnvalue_6 (- _returnvalue_5 (Math|Vector|MakeVector (.x _returnvalue_2) (.y _returnvalue_2) (.z _returnvalue_2))))
  (:Started
    (Development|PrintString "UpTrigger")
    (if (Variables|/Game/VRTemplate/Blueprints/GrabComponent.GrabComponent_C|GetbIsHeld (Variables|Default|GetWandGrabComponent))
      (bind _returnvalue_7 (Game|SpawnActorfromClass "/Game/Custom_BP/BP_Shootable.BP_Shootable_C" (Math|Transform|MakeTransform _returnvalue_5 "0, 0, 0" "0.300000,0.300000,0.300000") "Undefined" "MultiplyWithRoot" 0 0))
      (Physics|AddImpulse (Variables|/Game/Custom_BP/BP_Shootable.BP_Shootable_C|GetStaticMesh _returnvalue_7) (Math|Vector|MakeVector (* (.x _returnvalue_6) 2e+01) (* (.y _returnvalue_6) 2e+01) (* (.z _returnvalue_6) 2e+01)) "None" false))))

(event EventBeginPlay
  (bind _asvrpawn (Utilities|Casting|CastToVRPawn (Game|Player|GetPlayerPawn 0)))
  (Variables|Default|SetAs%20VRPawn _asvrpawn)
  (Rendering|SetVisibility (Variables|Default|GetNS_WandEnd) false false))

(event Collision|EventActorBeginOverlap
  (params (OtherActor :type Actor%20Object%20Reference)))

(event EventTick
  (params (DeltaSeconds :type Float%20%28single-precision%29))
  (bind _staticmesh_rootcomponent_ (Variables|Default|GetStaticMesh%28RootComponent%29))
  (bind _returnvalue (Transformation|GetWorldLocation _staticmesh_rootcomponent_))
  ;[1 1 1] Spawning objects and effects
  (if (Variables|/Game/VRTemplate/Blueprints/GrabComponent.GrabComponent_C|GetbIsHeld (Variables|Default|GetWandGrabComponent))
    (bind (_outhit _returnvalue_2) (Collision|LineTraceByChannel _returnvalue (+ _returnvalue (* (Transformation|GetWorldRotation _staticmesh_rootcomponent_) -2e+03)) "TraceTypeQuery1" false 0 "None"))
    (CallFunction|SpawnEffect (.location _outhit) _returnvalue_2)
    ;[1 1 1] Set Time
    (Utilities|IsValid (.hitcomponent _outhit)
      (:Is%20Valid
        (if (Utilities|Enum|Equal(Enum) (Utilities|GetObjectName (.hitcomponent _outhit)) "Torus")
          (CallFunction|SetTime (.location _outhit) (.hitcomponent _outhit))
          (Variables|/Game/Custom_BP/GameControllerComponent.GameControllerComponent_C|SetPlay (Variables|/Game/VRTemplate/Blueprints/VRPawn.VRPawn_C|GetGameControllerComponent (Variables|Default|GetAs%20VRPawn)) false)
          (else
            (Variables|/Game/Custom_BP/GameControllerComponent.GameControllerComponent_C|SetPlay (Variables|/Game/VRTemplate/Blueprints/VRPawn.VRPawn_C|GetGameControllerComponent (Variables|Default|GetAs%20VRPawn)) true)))))
    (else
      (Rendering|SetVisibility (Variables|Default|GetNS_WandEnd) false false))))

(fn ConstructionScript)

(fn SpawnObject
  (params (SpawnPointTransfrom :type Transform))
  (if (Variables|/Game/VRTemplate/Blueprints/VRPawn.VRPawn_C|GetisLeftIndexCurlTriggered (Variables|Default|GetAs%20VRPawn))
    (if (Variables|Default|GetbCanSpawnSoundObjectFlag)
      (Variables|Default|SetbCanSpawnSoundObjectFlag false)
      (bind _returnvalue (Game|SpawnActorfromClass "/Game/Custom_BP/BP_SoundObject.BP_SoundObject_C" SpawnPointTransfrom "Undefined" "MultiplyWithRoot" 0 0))
      (Physics|SetSimulatePhysics (Variables|/Game/Custom_BP/BP_SoundObject.BP_SoundObject_C|GetMesh _returnvalue) true)
      (switch int (Math|Conversions|ToInteger(Byte) (Variables|/Game/Custom_BP/GameControllerComponent.GameControllerComponent_C|GetMeshIndex (Variables|/Game/VRTemplate/Blueprints/VRPawn.VRPawn_C|GetGameControllerComponent (Variables|Default|GetAs%20VRPawn))))
        (:Default
          (Components|StaticMesh|SetStaticMesh (Variables|/Game/Custom_BP/BP_SoundObject.BP_SoundObject_C|GetMesh _returnvalue) "/Game/LevelPrototyping/Meshes/SM_Cube.SM_Cube")
          (Rendering|Material|SetMaterial (Variables|/Game/Custom_BP/BP_SoundObject.BP_SoundObject_C|GetMesh _returnvalue) 0 "/Game/FPWeapon/Materials/BaseMaterial.BaseMaterial"))
        (:0
          (Components|StaticMesh|SetStaticMesh (Variables|/Game/Custom_BP/BP_SoundObject.BP_SoundObject_C|GetMesh _returnvalue) "/Game/Megascans/3D_Assets/Cactus_udugdfvfa/S_Cactus_udugdfvfa_lod3_Var1.S_Cactus_udugdfvfa_lod3_Var1")
          (Rendering|Material|SetMaterial (Variables|/Game/Custom_BP/BP_SoundObject.BP_SoundObject_C|GetMesh _returnvalue) 0 "/Game/Megascans/3D_Assets/Cactus_udugdfvfa/MI_Cactus_udugdfvfa_2K.MI_Cactus_udugdfvfa_2K"))
        (:1
          (Components|StaticMesh|SetStaticMesh (Variables|/Game/Custom_BP/BP_SoundObject.BP_SoundObject_C|GetMesh _returnvalue) "/Game/Megascans/3D_Assets/Urban_Street_Pavestone_Gray_Single_xbyjdgh/S_Urban_Street_Pavestone_Gray_Single_xbyjdgh_lod3_Var1.S_Urban_Street_Pavestone_Gray_Single_xbyjdgh_lod3_Var1")
          (Rendering|Material|SetMaterial (Variables|/Game/Custom_BP/BP_SoundObject.BP_SoundObject_C|GetMesh _returnvalue) 0 "/Game/Megascans/3D_Assets/Urban_Street_Pavestone_Gray_Single_xbyjdgh/MI_Urban_Street_Pavestone_Gray_Single_xbyjdgh_2K.MI_Urban_Street_Pavestone_Gray_Single_xbyjdgh_2K"))
        (:2
          (Components|StaticMesh|SetStaticMesh (Variables|/Game/Custom_BP/BP_SoundObject.BP_SoundObject_C|GetMesh _returnvalue) "/Game/Megascans/3D_Assets/Japanese_Mossy_Stone_Wall_ulldfgb/S_Japanese_Mossy_Stone_Wall_ulldfgb_lod3.S_Japanese_Mossy_Stone_Wall_ulldfgb_lod3")
          (Rendering|Material|SetMaterial (Variables|/Game/Custom_BP/BP_SoundObject.BP_SoundObject_C|GetMesh _returnvalue) 0 "/Game/Megascans/3D_Assets/Japanese_Mossy_Stone_Wall_ulldfgb/MI_Japanese_Mossy_Stone_Wall_ulldfgb_2K.MI_Japanese_Mossy_Stone_Wall_ulldfgb_2K"))))
    (else
      (Variables|Default|SetbCanSpawnSoundObjectFlag true))))

(fn SpawnEffect
  (params (HitPoint :type Vector) (Hit :type Boolean))
  (bind _ns_wandend (Variables|Default|GetNS_WandEnd))
  (if Hit
    (Rendering|SetVisibility _ns_wandend true false)
    (Transformation|SetWorldLocation _ns_wandend HitPoint false false)
    (else
      (Rendering|SetVisibility _ns_wandend false false))))

(fn SetTime
  (params (HitPoint :type Vector) (OtherComponent :type Scene%20Component%20Object%20Reference))
  (bind _returnvalue (Transformation|GetWorldLocation OtherComponent))
  (bind _as_vrpawn (Variables|Default|GetAs%20VRPawn))
  (bind _returnvalue_2 (- HitPoint _returnvalue))
  (bind _gamecontrollercomponent (Variables|/Game/VRTemplate/Blueprints/VRPawn.VRPawn_C|GetGameControllerComponent _as_vrpawn))
  (bind _returnvalue_3 (/ (.y _returnvalue_2) (.x _returnvalue_2)))
  (bind _songlength (Variables|/Game/Custom_BP/GameControllerComponent.GameControllerComponent_C|GetSongLength _gamecontrollercomponent))
  (bind _returnvalue_4 (Class|KismetMathLibrary|DegAtan _returnvalue_3))
  (bind _returnvalue_5 (/ _songlength 2.0))
  (bind _returnvalue_6 (/ _returnvalue_4 3.6e+02))
  (bind _returnvalue_7 (* _returnvalue_6 _songlength))
  (if (> (.x _returnvalue_2) 0.0)
    ;[1 1 1] x > 0
    (Variables|/Game/Custom_BP/GameControllerComponent.GameControllerComponent_C|SetPlayTime _gamecontrollercomponent _returnvalue_7)
    (elif (< (.x _returnvalue_2) 0.0)
      ;[1 1 1] x < 0
      (if (< _returnvalue_7 (/ _songlength 4.0))
        (Variables|/Game/Custom_BP/GameControllerComponent.GameControllerComponent_C|SetPlayTime _gamecontrollercomponent (+ _returnvalue_7 _returnvalue_5))
        (elif (> (* (/ _songlength 4.0) 3.0) _songlength)
          (Variables|/Game/Custom_BP/GameControllerComponent.GameControllerComponent_C|SetPlayTime _gamecontrollercomponent (- _returnvalue_7 _returnvalue_5)))))))