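; BP_PlayBar is a playback indicator that moves its PlayBar component around a horizontal circle to show song progress.
; BeginPlay places the bar at the circle's starting point and caches the player's VRPawn.
; Each Tick converts the ratio of PlayTime to SongLength from the pawn's GameControllerComponent into an angle, using cosine and sine to set the relative location, so one full lap spans the song.
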(event EventBeginPlay
  (Transformation|SetRelativeLocation (Variables|Default|GetPlayBar) "300.000000,0.000000,0.000000" false false)
  (bind _asvrpawn (Utilities|Casting|CastToVRPawn (Game|Player|GetPlayerPawn 0)))
  (Variables|Default|SetAs%20VRPawn _asvrpawn))

(event Collision|EventActorBeginOverlap
  (params (OtherActor :type Actor%20Object%20Reference)))

(event EventTick
  (params (DeltaSeconds :type Float%20%28single-precision%29))
  (bind _as_vrpawn (Variables|Default|GetAs%20VRPawn))
  (bind _gamecontrollercomponent (Variables|/Game/VRTemplate/Blueprints/VRPawn.VRPawn_C|GetGameControllerComponent _as_vrpawn))
  (bind _songlength (Variables|/Game/Custom_BP/GameControllerComponent.GameControllerComponent_C|GetSongLength _gamecontrollercomponent))
  (bind _playtime (Variables|/Game/Custom_BP/GameControllerComponent.GameControllerComponent_C|GetPlayTime _gamecontrollercomponent))
  (bind _returnvalue (/ _playtime _songlength))
  (bind _returnvalue_2 (* _returnvalue 3.6e+02))
  (Transformation|SetRelativeLocation (Variables|Default|GetPlayBar) (* (Math|Vector|MakeVector (Math|Trig|Cos(Degrees) _returnvalue_2) (Math|Trig|Sin(Degrees) _returnvalue_2) 0.0) "300.000000,300.000000,0.000000") false false))

(fn ConstructionScript)