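; BP_Recorder is a VR record button that toggles audio recording whenever something overlaps its box.
; Starting updates the text label, resets PlayTime on the VR pawn's GameControllerComponent, starts AudioCapture and begins recording audio output.
; The next overlap stops both and exports the result as a WAV file named FinalScore.
; The overlap is not filtered by actor, so any overlapping object flips the state.
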(event OnComponentBeginOverlap(Box)
  (params (OverlappedComponent :type Primitive%20Component%20Object%20Reference) (OtherActor :type Actor%20Object%20Reference) (OtherComp :type Primitive%20Component%20Object%20Reference) (OtherBodyIndex :type Integer) (bFromSweep :type Boolean) (SweepResult :type Hit%20Result%20Structure%20%28by%20ref%29))
  (bind _audiocapture (Variables|Default|GetAudioCapture))
  (if (Variables|Default|GetRecording)
    (Variables|Default|SetRecording false)
    (Class|Text3DComponent|SetText (Variables|Default|GetRecordText) (Utilities|Text|FormatText "Record"))
    (Audio|Components|Audio|Stop _audiocapture)
    (Class|AudioMixerBlueprintLibrary|StopRecordingOutput "WavFile" "FinalScore" "" 0 0)
    (else
      (Variables|Default|SetRecording true)
      (Class|Text3DComponent|SetText (Variables|Default|GetRecordText) (Utilities|Text|FormatText "Recording..."))
      (Variables|/Game/Custom_BP/GameControllerComponent.GameControllerComponent_C|SetPlayTime (Variables|/Game/VRTemplate/Blueprints/VRPawn.VRPawn_C|GetGameControllerComponent (Variables|Default|GetAs%20VRPawn)) 0.0)
      (CameraShake|Start _audiocapture)
      (Class|AudioMixerBlueprintLibrary|StartRecordingOutput 0.0 0))))

(event EventBeginPlay
  (bind _asvrpawn (Utilities|Casting|CastToVRPawn (Game|Player|GetPlayerPawn 0)))
  (Variables|Default|SetAs%20VRPawn _asvrpawn))

(fn ConstructionScript)