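; BP_ReplaySoundObject is a short-lived actor that plays a one-shot sound, named for use with replays.
; Its Play function plays the stored Sound at the stored Location and Pitch; nothing in the actor calls it.
; Tick accumulates delta time in Timer and destroys the actor after about two seconds, whether or not Play has run.
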(event EventBeginPlay)

(event Collision|EventActorBeginOverlap
  (params (OtherActor :type Actor%20Object%20Reference)))

(event EventTick
  (params (DeltaSeconds :type Float%20%28single-precision%29))
  (bind _output_get (Variables|Default|Settimer (+ DeltaSeconds (Variables|Default|Gettimer))))
  (if (>= _output_get 2.0)
    (Actor|DestroyActor)))

(fn ConstructionScript)

(fn Play
  (Audio|PlaySoundatLocation (Variables|Default|GetSound) (Variables|Default|Getlocation) "0, 0, 0" 1.0 (Variables|Default|GetPitch) 0.0 0 0 0 0))